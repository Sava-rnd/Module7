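; Traffic light actor that endlessly cycles green, yellow, red, yellow and back to green from BeginPlay.
; A chain of timed delays calls a turn function for each color, then fires LightChange to loop back to the first delay.
; Each turn function lights one lamp with its color material and sets the other two to LightMaterial.
; The first green wait runs without calling TurnGreen, so it relies on the initial materials.
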(event Custom|LightChange
  (Utilities|FlowControl|Delay (Variables|Default|GetGreen%20))
  (CallFunction|TurnYellow)
  (Utilities|FlowControl|Delay (Variables|Default|GetYellow%20))
  (CallFunction|TurnRed)
  (Utilities|FlowControl|Delay (Variables|Default|GetRed%20))
  (CallFunction|TurnYellow)
  (Utilities|FlowControl|Delay (Variables|Default|GetYellow%20))
  (CallFunction|TurnGreen)
  (CallFunction|LightChange))

(event EventBeginPlay
  (Utilities|FlowControl|Delay (Variables|Default|GetGreen%20))
  (CallFunction|TurnYellow)
  (Utilities|FlowControl|Delay (Variables|Default|GetYellow%20))
  (CallFunction|TurnRed)
  (Utilities|FlowControl|Delay (Variables|Default|GetRed%20))
  (CallFunction|TurnYellow)
  (Utilities|FlowControl|Delay (Variables|Default|GetYellow%20))
  (CallFunction|TurnGreen)
  (CallFunction|LightChange))

(event Collision|EventActorBeginOverlap
  (params (OtherActor :type Actor%20Object%20Reference)))

(event EventTick
  (params (DeltaSeconds :type Float%20%28single-precision%29)))

(fn ConstructionScript)

(fn TurnGreen
  (Rendering|Material|SetMaterial (Variables|Default|GetGreen) 0 "/Game/Module/Blueprints/Material/GreenMaterial.GreenMaterial")
  (Rendering|Material|SetMaterial (Variables|Default|GetYellow) 0 "/Game/Module/Blueprints/Material/LightMaterial.LightMaterial")
  (Rendering|Material|SetMaterial (Variables|Default|GetRed) 0 "/Game/Module/Blueprints/Material/LightMaterial.LightMaterial"))

(fn TurnYellow
  (Rendering|Material|SetMaterial (Variables|Default|GetGreen) 0 "/Game/Module/Blueprints/Material/LightMaterial.LightMaterial")
  (Rendering|Material|SetMaterial (Variables|Default|GetYellow) 0 "/Game/Module/Blueprints/Material/YellowMaterial.YellowMaterial")
  (Rendering|Material|SetMaterial (Variables|Default|GetRed) 0 "/Game/Module/Blueprints/Material/LightMaterial.LightMaterial"))

(fn TurnRed
  (Rendering|Material|SetMaterial (Variables|Default|GetGreen) 0 "/Game/Module/Blueprints/Material/LightMaterial.LightMaterial")
  (Rendering|Material|SetMaterial (Variables|Default|GetYellow) 0 "/Game/Module/Blueprints/Material/LightMaterial.LightMaterial")
  (Rendering|Material|SetMaterial (Variables|Default|GetRed) 0 "/Game/Module/Blueprints/Material/RedMaterial.RedMaterial"))